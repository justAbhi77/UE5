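; BP_WhiteHole is a white hole actor that repels physics objects within its influence range.
; Every tick, ApplyForces finds components overlapping GravityInfluenceRange and pushes those simulating physics directly away from the actor.
; The push weakens linearly as scaled distance grows until it reaches a clamp, and is scaled by GravityStrength and multiplier variables.
; It is applied as an acceleration change, so mass does not affect the result.
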(event EventBeginPlay)

(event Collision|EventActorBeginOverlap
  (params (OtherActor :type Actor%20Object%20Reference)))

(event EventTick
  (params (DeltaSeconds :type Float%20%28single-precision%29))
  (CallFunction|ApplyForces))

(fn ConstructionScript)

(fn ApplyForces
  (bind _returnvalue (Transformation|GetActorLocation))
  (for _array_element (Class|PrimitiveComponent|GetOverlappingComponents (Variables|Default|GetGravityInfluenceRange))
    (if (Physics|IsSimulatingPhysics _array_element "None")
      (Physics|AddForce _array_element (* (* (Math|Vector|GetUnitDirection(Vector) (Transformation|GetWorldLocation _array_element) _returnvalue) (* (- (Variables|Public|GetClampMaxValue) (Math|Float|Clamp(Float) (/ (Math|Vector|Distance(Vector) _returnvalue (Transformation|GetWorldLocation _array_element)) (Variables|Public|GetDistanceDiviser)) 0.0 (Variables|Public|GetClampMaxValue))) (Variables|Public|GetDistanceMultiplier)) (Variables|Public|GetVector3Multiplier) (Variables|Public|GetGravityStrength)) -1.0) "None" true))))