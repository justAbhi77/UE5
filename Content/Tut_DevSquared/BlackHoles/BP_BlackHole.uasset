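; Black hole actor that pulls in physics objects and either swallows them or sends them to a linked white hole.
; Each tick, it accelerates simulating components within its influence range toward its center, more strongly when closer.
; Physics objects entering the kill zone teleport to the white hole with clamped mesh velocity, if one is linked.
; Otherwise they are destroyed and their mass grows the sphere through a timeline-driven scale.
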(event OnComponentBeginOverlap(Killzone)
  (params (OverlappedComponent :type Primitive%20Component%20Object%20Reference) (OtherActor :type Actor%20Object%20Reference) (OtherComp :type Primitive%20Component%20Object%20Reference) (OtherBodyIndex :type Integer) (bFromSweep :type Boolean) (SweepResult :type Hit%20Result%20Structure%20%28by%20ref%29))
  (if (Physics|IsSimulatingPhysics OtherComp "None")
    (if (Utilities|IsValid (Variables|Public|GetLinkedWhiteHole))
      (CallFunction|TeleportActor OtherActor)
      (else
        (CallFunction|MassGained (Physics|GetMass OtherComp))
        (Actor|DestroyActor OtherActor)))))

(event Custom|MassGained
  (params (Mass :type Float%20%28double-precision%29))
  (Variables|Private|SetCurrentScale (Transformation|GetWorldScale (Variables|Default|GetSphere)))
  (Variables|Private|SetNewScale (+ (Variables|Private|GetCurrentScale) (* Mass (Variables|Public|GetGrowthRateMultiplier))))
  (bind _delta (Timeline|Timeline PlayFromStart)
    (:Update
      (Transformation|SetWorldScale3D (Variables|Default|GetSphere) (Math|Interpolation|Ease "Linear" _delta (Variables|Private|GetCurrentScale) (Variables|Private|GetNewScale))))))

(event EventBeginPlay)

(event Collision|EventActorBeginOverlap
  (params (OtherActor :type Actor%20Object%20Reference)))

(event EventTick
  (params (DeltaSeconds :type Float%20%28single-precision%29))
  (CallFunction|ApplyForces))

(fn ConstructionScript)

(fn ApplyForces
  (bind _returnvalue (Transformation|GetActorLocation))
  (for _array_element (Class|PrimitiveComponent|GetOverlappingComponents (Variables|Default|GetGravityInfluenceRange))
    (if (Physics|IsSimulatingPhysics _array_element "None")
      (Physics|AddForce _array_element (* (Math|Vector|GetUnitDirection(Vector) (Transformation|GetWorldLocation _array_element) _returnvalue) (* (- (Variables|Public|GetClampMaxValue) (Math|Float|Clamp(Float) (/ (Math|Vector|Distance(Vector) _returnvalue (Transformation|GetWorldLocation _array_element)) (Variables|Public|GetDistanceDiviser)) 0.0 (Variables|Public|GetClampMaxValue))) (Variables|Public|GetDistanceMultiplier)) (Variables|Public|GetVector3Multiplier) (Variables|Public|GetGravityStrength)) "None" true))))

(fn TeleportActor
  (params (Actor :type Actor%20Object%20Reference))
  (Transformation|SetActorLocation Actor (Transformation|GetActorLocation (Variables|Public|GetLinkedWhiteHole)) false false)
  (for _array_element (Actor|GetComponentsByClass Actor "/Script/Engine.StaticMeshComponent")
    (if (Physics|IsSimulatingPhysics _array_element "None")
      (bind _returnvalue (Physics|GetPhysicsLinearVelocity _array_element "None"))
      (Physics|SetPhysicsLinearVelocity _array_element (Math|Vector|ClampVectorSize _returnvalue 0.0 (Variables|Public|GetMaxVelocityClamp)) false "None"))))