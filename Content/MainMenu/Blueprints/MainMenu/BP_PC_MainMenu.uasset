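; Main menu player controller that manages the menu's UI screens and shows the main menu widget on Begin Play.
; A ShowHideWidgets event takes a widget enum and a show flag and routes to show or hide functions that switch on the enum.
; Main Menu and Create Server widgets are created on first show, cached, then added to or removed from the viewport.
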(event Custom|ShowHideWidgets
  (params (Widget :type E_MainMenuWidget%20Enum :default "NewEnumerator0") (Show? :type Boolean))
  ;[1 1 1] Show Hide Widgets
  (if Show?
    (CallFunction|FShowWidgets Widget)
    (else
      (CallFunction|FHideWidgets Widget))))

(event EventBeginPlay
  ;[1 1 1] Begin Play
  (CallFunction|ShowHideWidgets "NewEnumerator0" true))

(fn ConstructionScript)

(fn FShowWidgets
  (params (Widget :type E_MainMenuWidget%20Enum :default "NewEnumerator0"))
  (switch Utilities|FlowControl|Switch|SwitchonE_MainMenuWidget Widget
    (:NewEnumerator0
      (Variables|Default|GetWB_MainMenu
        (:then
          _)
        (:else
          (bind _returnvalue (UserInterface|CreateWidget "/Game/MainMenu/UI/MainMenu/WBP_MainMenu.WBP_MainMenu_C"))
          (bind _output_get (Variables|Default|SetWB_MainMenu _returnvalue))))
      (UserInterface|Viewport|AddtoViewport _output_get 0))
    (:NewEnumerator1
      (Variables|Default|GetWB_CreateServer
        (:then
          _)
        (:else
          (bind _returnvalue_2 (UserInterface|CreateWidget "/Game/MainMenu/UI/MainMenu/WBP_CreateServer.WBP_CreateServer_C"))
          (bind _output_get_2 (Variables|Default|SetWB_CreateServer _returnvalue_2))))
      (UserInterface|Viewport|AddtoViewport _output_get_2 0))))

(fn FHideWidgets
  (params (Widget :type E_MainMenuWidget%20Enum :default "NewEnumerator0"))
  (switch Utilities|FlowControl|Switch|SwitchonE_MainMenuWidget Widget
    (:NewEnumerator0
      (bind _wb_mainmenu (Variables|Default|GetWB_MainMenu)
        (:then
          (Widget|RemovefromParent _wb_mainmenu))
        (:else)))
    (:NewEnumerator1
      (bind _wb_createserver (Variables|Default|GetWB_CreateServer)
        (:then
          (Widget|RemovefromParent _wb_createserver))
        (:else)))))

(fn GetPlayerControllerRef
  (return self))