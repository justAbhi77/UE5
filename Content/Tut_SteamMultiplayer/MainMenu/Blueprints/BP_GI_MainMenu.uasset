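; Main menu Game Instance that hosts multiplayer games through Advanced Sessions.
; CreateServer creates a session with the given slot count and LAN flag, advertising server name, map, language and LAN as extra settings.
; On success it opens the level matching SelectedGameMap as a listen server; only FirstPersonMap is mapped.
; GetGameInstaneRef returns the instance itself.
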(event Custom|CreateServer
  (params (ServerName :type String) (AmountOfSlots :type Integer) (ServerLanguage :type String) (bUseLAN :type Boolean))
  (|AdvancedSession (Utilities|Array|MakeArray (Class|AdvancedSessionsLibrary|MakeLiteralSessionPropertyString "ServerName" ServerName) (Class|AdvancedSessionsLibrary|MakeLiteralSessionPropertyString "ServerMap" (Utilities|String|EnumtoString (Variables|Default|GetSelectedGameMap))) (Class|AdvancedSessionsLibrary|MakeLiteralSessionPropertyString "ServerLanguage" ServerLanguage) (Class|AdvancedSessionsLibrary|MakeLiteralSessionPropertyBool "UseLan" bUseLAN)) (Game|GetPlayerController 0) AmountOfSlots 0 bUseLAN true false true true true false false false true false true
    (:OnSuccess
      (Game|OpenLevel(byObjectReference) (Utilities|Select :Index (Variables|Default|GetSelectedGameMap) :NewEnumerator0 "/Game/FirstPerson/Maps/FirstPersonMap.FirstPersonMap") true "listen"))))

(fn GetGameInstaneRef
  (return self))